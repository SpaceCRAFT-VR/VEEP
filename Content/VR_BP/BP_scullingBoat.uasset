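; Sculling boat Blueprint that detects water bodies overlapping its capsule and spawns splash particles at the surface.
; BeginPlay caches all WaterBody actors, which a delayed Tick loop tests to track the current overlap.
; Splashes spawn only at low WaterLevelAlpha, use the water plane's height, get a water tag and take their color from the body's tag.
; FireWaterSplash shares that spawn path, but its foot-hit binding and speed gate are unconnected.
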(event Custom|FireWaterSplash
  (bind _watertag (Variables|Default|GetWaterTag))
  (bind _capsule (Variables|Default|GetCapsule))
  (bind _returnvalue (Transformation|GetWorldLocation _capsule))
  ;[1 1 1] Run animation has a notify ("splash") -> In AnimBp this notify is an event -> this event is called via event dispatcher in ThirdPerson_BP -> now splash can be controlled
  ;[1 1 1] on splash event-> then get its height to spawn splash always at water surface Z + character location
  (if (<= (Variables|Default|GetWaterLevelAlpha) 5e+01)
    (bind _returnvalue_2 (Effects|SpawnEmitteratLocation "/Game/_Marvelmaster_infinite_reactive_water_/Particles/Splash_PS.Splash_PS" (Math|Vector|MakeVector (.x _returnvalue) (.y _returnvalue) (.z (Transformation|GetWorldLocation (Variables|Default|GetWaterPlane))))))
    ;[1 1 1] Set tag of spawned particle to "water"
    (Variables|/Script/Engine.Actor|SetTags (Components|GetOwner _returnvalue_2) _watertag)
    (Variables|/Script/Engine.ActorComponent|SetComponentTags _returnvalue_2 _watertag)
    ;[1 1 1] change water splash color by water body tag
    (switch string (Utilities|String|ToString(Name) (Utilities|Array|Get(acopy) (Variables|/Script/Engine.Actor|GetTags (Components|GetOwner (Variables|Default|GetOverlappingWaterBody)))))
      (:Default
        (Effects|Components|ParticleSystem|SetColorParameter _returnvalue_2 "color" "(R=0.568627,G=0.921569,B=0.980392,A=1.000000)" :!label _label))
      (:red
        (Effects|Components|ParticleSystem|SetColorParameter _returnvalue_2 "color" "(R=1.000000,G=0.015686,B=0.000000,A=1.000000)"))
      (:green
        (Effects|Components|ParticleSystem|SetColorParameter _returnvalue_2 "color" "(R=0.086275,G=0.615686,B=0.000000,A=1.000000)"))
      (:blue
        (goto _label)))))

(event EventTick
  (params (DeltaSeconds :type Float%20%28single-precision%29))
  (bind _watertag (Variables|Default|GetWaterTag))
  (bind _capsule (Variables|Default|GetCapsule))
  (bind _returnvalue (Transformation|GetWorldLocation _capsule))
  ;[1 1 1] Check if character is overlapping water surface
  (Utilities|FlowControl|Delay 0.1)
  (for _array_element (Variables|Default|GetValidWaterBodies)
    (Utilities|FlowControl|Sequence
      (:then_0
        (if (Class|PrimitiveComponent|IsOverlappingComponent (Variables|/Game/_Marvelmaster_infinite_reactive_water_/Blueprints/WaterBody_BP0.WaterBody_BP0_C|GetOverlapBox _array_element) (Variables|Default|GetCapsule))
          (Variables|Default|SetWaterPlane (Variables|/Game/_Marvelmaster_infinite_reactive_water_/Blueprints/WaterBody_BP0.WaterBody_BP0_C|GetWaterPlaneMesh _array_element))
          (bind _output_get (Variables|Default|SetOverlappingWaterBody (Variables|/Game/_Marvelmaster_infinite_reactive_water_/Blueprints/WaterBody_BP0.WaterBody_BP0_C|GetOverlapBox _array_element)))
          ;[1 1 1] on splash event-> then get its height to spawn splash always at water surface Z + character location
          (if (<= (Variables|Default|GetWaterLevelAlpha) 5e+01) :!label _label
            (bind _returnvalue_2 (Effects|SpawnEmitteratLocation "/Game/_Marvelmaster_infinite_reactive_water_/Particles/Splash_PS.Splash_PS" (Math|Vector|MakeVector (.x _returnvalue) (.y _returnvalue) (.z (Transformation|GetWorldLocation (Variables|Default|GetWaterPlane))))))
            ;[1 1 1] Set tag of spawned particle to "water"
            (Variables|/Script/Engine.Actor|SetTags (Components|GetOwner _returnvalue_2) _watertag)
            (Variables|/Script/Engine.ActorComponent|SetComponentTags _returnvalue_2 _watertag)
            ;[1 1 1] change water splash color by water body tag
            (switch string (Utilities|String|ToString(Name) (Utilities|Array|Get(acopy) (Variables|/Script/Engine.Actor|GetTags (Components|GetOwner (Variables|Default|GetOverlappingWaterBody)))))
              (:Default
                (Effects|Components|ParticleSystem|SetColorParameter _returnvalue_2 "color" "(R=0.568627,G=0.921569,B=0.980392,A=1.000000)" :!label _label_2))
              (:red
                (Effects|Components|ParticleSystem|SetColorParameter _returnvalue_2 "color" "(R=1.000000,G=0.015686,B=0.000000,A=1.000000)"))
              (:green
                (Effects|Components|ParticleSystem|SetColorParameter _returnvalue_2 "color" "(R=0.086275,G=0.615686,B=0.000000,A=1.000000)"))
              (:blue
                (goto _label_2))))
          (elif (Utilities|IsValid (Variables|Default|GetOverlappingWaterBody))
            (if (not (Class|PrimitiveComponent|IsOverlappingComponent _output_get (Variables|Default|GetCapsule)))
              (Variables|Default|SetOverlappingWaterBody 0)
              (goto _label))))))))

(event EventBeginPlay
  (Utilities|FlowControl|Sequence
    (:then_0
      ;[1 1 1] Run animation has a notify ("splash") -> In AnimBp this notify is an event -> this event is called via event dispatcher in ThirdPerson_BP -> now splash can be controlled
      (bind _outactors (Actor|GetAllActorsOfClass "/Game/_Marvelmaster_infinite_reactive_water_/Blueprints/WaterBody_BP0.WaterBody_BP0_C"))
      (Variables|Default|SetValidWaterBodies _outactors))
    (:then_1
      (Development|ExecuteConsoleCommand "disableallscreenmessages" 0))))

(event Collision|EventActorBeginOverlap
  (params (OtherActor :type Actor%20Object%20Reference)))

(fn ConstructionScript)